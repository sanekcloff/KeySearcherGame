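; BP_Key is a key actor that spins in place and vanishes when something overlaps it.
; BeginPlay picks a random spin direction, and Tick applies a local yaw rotation in that direction each frame.
; On any actor overlap it casts the game mode to BP_KSGameModeBase and destroys itself if that succeeds, without using the game mode further.
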(event EventBeginPlay
  (if (Math|Random|RandomBool)
    (Variables|Default|SetDirection -1.0)
    (else
      (Variables|Default|SetDirection 1.0))))

(event Collision|EventActorBeginOverlap
  (params (OtherActor :type Actor%20Object%20Reference))
  (Utilities|Casting|CastToBP_KSGameModeBase (Game|GetGameMode))
  (Actor|DestroyActor))

(event EventTick
  (params (DeltaSeconds :type Float%20%28single-precision%29))
  (Transformation|AddActorLocalRotation (Math|Rotator|MakeRotator 0.0 0.0 (* (Variables|Default|GetRotationYaw) (Variables|Default|GetDirection))) false false))

(fn ConstructionScript)